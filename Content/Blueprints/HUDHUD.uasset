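; HUD Blueprint that draws a multiplayer main menu with an IP entry field and a lobby screen with host-only Start and Quit buttons.
; DrawHUD renders screens from state flags, using a DrawButton helper that adds a named hit box per button.
; Number, period and delete keys edit the IP string.
; Hit box clicks set pressed textures, while releases build console commands to host, join, server-travel or exit.
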(event EventBeginPlay)

(event EventActorBeginOverlap
  (params (OtherActor :type Actor%20Object%20Reference)))

(event EventTick
  (params (DeltaSeconds :type Float%20%28single-precision%29)))

(event EventDrawHUD
  (params (SizeX :type Integer) (SizeY :type Integer))
  (bind _returnvalue (Math|Float|MakeLiteralFloat 3.5e+02))
  (bind _returnvalue_2 (Math|Float|MakeLiteralFloat 4.5e+02))
  (bind _buttontexture (Variables|Default|GetButtonTexture))
  (Variables|Default|SetButtonSize (Math|Vector2D|MakeVector2D (Math|Conversions|ToFloat(Integer) (Class|Texture2D|BlueprintGetSizeX _buttontexture)) (Math|Conversions|ToFloat(Integer) (Class|Texture2D|BlueprintGetSizeY _buttontexture))))
  (Variables|Default|SetScreenDimensions (Math|Vector2D|MakeVector2D (Math|Conversions|ToFloat(Integer) SizeX) (Math|Conversions|ToFloat(Integer) SizeY)))
  (if (Variables|Default|GetMainMenuActive)
    (Class|HUD|DrawMaterialSimple "/Game/Blueprints/MenuBackground_Mat.MenuBackground_Mat" 0.0 0.0 (.X (Math|Vector2D|BreakVector2D (Variables|Default|GetScreenDimensions))) (.Y (Math|Vector2D|BreakVector2D (Variables|Default|GetScreenDimensions))) 1.0 false)
    (HUD|DrawRect (Variables|Default|GetTextBackgroundColor) _returnvalue_2 _returnvalue (Math|Float|MakeLiteralFloat 7e+02) (Math|Float|MakeLiteralFloat 1e+02))
    (HUD|DrawText (Variables|Default|GetipString) (Variables|Default|GetTextColor) _returnvalue_2 _returnvalue "/Game/Blueprints/NewFont.NewFont" 2.0 false)
    (CallFunction|DrawButton (Math|Vector2D|MakeVector2D 1e+01 2e+02) (Variables|Default|GetButtonSize) "Host" (select (Variables|Default|GetHostButtonPressed) (Variables|Default|GetButtonTexturePressed) (Variables|Default|GetButtonTexture)) (Variables|Default|GetTextColor))
    (CallFunction|DrawButton (Math|Vector2D|MakeVector2D 1e+01 3e+02) (Variables|Default|GetButtonSize) "Join" (select (Variables|Default|GetJoinButtonPressed) (Variables|Default|GetButtonTexturePressed) (Variables|Default|GetButtonTexture)) (Variables|Default|GetTextColor))
    (CallFunction|DrawButton (Math|Vector2D|MakeVector2D 1e+01 4e+02) (Variables|Default|GetButtonSize) "Quit" (select (Variables|Default|GetQuitButtonPressed) (Variables|Default|GetButtonTexturePressed) (Variables|Default|GetButtonTexture)) (Variables|Default|GetTextColor))
    (elif (Variables|Default|GetLobbyActive)
      (Class|HUD|DrawMaterialSimple "/Game/Blueprints/LobbyBackground_Mat.LobbyBackground_Mat" 0.0 0.0 (.X (Math|Vector2D|BreakVector2D (Variables|Default|GetScreenDimensions))) (.Y (Math|Vector2D|BreakVector2D (Variables|Default|GetScreenDimensions))) 1.0 false)
      (if (Variables|Default|GetIsHost)
        (CallFunction|DrawButton (Math|Vector2D|MakeVector2D 1e+01 3e+02) (Variables|Default|GetButtonSize) "Start" (select (Variables|Default|GetStartButtonPressed) (Variables|Default|GetButtonTexturePressed) (Variables|Default|GetButtonTexture)) (Variables|Default|GetTextColor))
        (CallFunction|DrawButton (Math|Vector2D|MakeVector2D 1e+01 4e+02) (Variables|Default|GetButtonSize) "Quit" (select (Variables|Default|GetQuitButtonPressed) (Variables|Default|GetButtonTexturePressed) (Variables|Default|GetButtonTexture)) (Variables|Default|GetTextColor))))))

(event EventHitBoxRelease
  (params (BoxName :type Name :default "None"))
  (bind _returnvalue (Utilities|String|MakeLiteralString "Travel "))
  (switch name BoxName
    (:Host
      (Development|ExecuteConsoleCommand (Utilities|String|Append _returnvalue (Utilities|String|MakeLiteralString "Lobby?Listen"))))
    (:Join
      (Development|ExecuteConsoleCommand (Utilities|String|Append _returnvalue (Variables|Default|GetipString))))
    (:Quit
      (Development|ExecuteConsoleCommand "Exit"))
    (:Start
      (Variables|Default|SetLobbyActive false)
      (Variables|Default|SetMainMenuActive false)
      (Development|ExecuteConsoleCommand (Utilities|String|Append (Utilities|String|MakeLiteralString "ServerTravel ") (Variables|Default|GetGameLevelName))))))

(event EventHitBoxClick
  (params (BoxName :type Name :default "None"))
  (switch name BoxName
    (:Host
      (Variables|Default|SetHostButtonPressed true))
    (:Join
      (Variables|Default|SetJoinButtonPressed true))
    (:Quit
      (Variables|Default|SetQuitButtonPressed true))
    (:Start
      (Variables|Default|SetStartButtonPressed true))))

(event Input|KeyboardEvents|1
  (:Pressed
    (CallFunction|BuildHostString "1")))

(event Input|KeyboardEvents|2
  (:Pressed
    (CallFunction|BuildHostString "2")))

(event Input|KeyboardEvents|3
  (:Pressed
    (CallFunction|BuildHostString "3")))

(event Input|KeyboardEvents|4
  (:Pressed
    (CallFunction|BuildHostString "4")))

(event Input|KeyboardEvents|5
  (:Pressed
    (CallFunction|BuildHostString "5")))

(event Input|KeyboardEvents|6
  (:Pressed
    (CallFunction|BuildHostString "6")))

(event Input|KeyboardEvents|7
  (:Pressed
    (CallFunction|BuildHostString "7")))

(event Input|KeyboardEvents|8
  (:Pressed
    (CallFunction|BuildHostString "8")))

(event Input|KeyboardEvents|9
  (:Pressed
    (CallFunction|BuildHostString "9")))

(event Input|KeyboardEvents|0
  (:Pressed
    (CallFunction|BuildHostString "0")))

(event Input|KeyboardEvents|Period
  (:Pressed
    (CallFunction|BuildHostString ".")))

(event Input|KeyboardEvents|Backspace
  (:Pressed
    (CallFunction|DeleteStringCharacter)))

(event Input|KeyboardEvents|Delete
  (:Pressed
    (CallFunction|DeleteStringCharacter)))

(event Input|MouseEvents|LeftMouseButton
  (:Released
    (Variables|Default|SetHostButtonPressed false)
    (Variables|Default|SetJoinButtonPressed false)
    (Variables|Default|SetQuitButtonPressed false)
    (Variables|Default|SetStartButtonPressed false)))

(fn ConstructionScript)

(fn DrawButton
  (params (ButtonScreenLocation :type Vector%202D%20Structure) (ButtonSize :type Vector%202D%20Structure) (ButtonText :type String) (Texture :type Texture%20Object%20Reference) (TextColor :type Linear%20Color%20Structure))
  (bind (_x _y) (Math|Vector2D|BreakVector2D ButtonScreenLocation))
  (bind (_outwidth _outheight) (Class|HUD|GetTextSize ButtonText 0 1.0))
  (bind _returnvalue (/ ButtonSize 4.0))
  (bind _returnvalue_2 (Math|Vector2D|MakeVector2D _outwidth _outheight))
  (bind _returnvalue_3 (+ _returnvalue ButtonScreenLocation))
  (bind _returnvalue_4 (/ _returnvalue_2 2.0))
  (bind _returnvalue_5 (- _returnvalue_3 _returnvalue_4))
  (bind (_x_2 _y_2) (Math|Vector2D|BreakVector2D _returnvalue_5))
  (Class|HUD|DrawTextureSimple Texture _x _y 1.0 false)
  (HUD|DrawText ButtonText "(R=0,G=0,B=0,A=1)" _x_2 _y_2 "/Game/Blueprints/NewFont.NewFont" 1.0 false)
  (Class|HUD|AddHitBox ButtonScreenLocation ButtonSize (Utilities|String|StringToName ButtonText) false))

(fn BuildHostString
  (params (Key%20Input :type String))
  (Variables|Default|SetipString (Utilities|String|Append (Variables|Default|GetipString) Key%20Input)))

(fn DeleteStringCharacter
  (Variables|Default|SetipString (Utilities|String|GetSubstring (Variables|Default|GetipString) 0 (- (Utilities|String|Len (Variables|Default|GetipString)) 1))))